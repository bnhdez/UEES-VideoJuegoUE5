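; BP_FinalNivel is the level-end trigger, finishing the level once enough coins are collected.
; When a character overlaps its Box, it asks GM_Programacion whether the coin requirement is met.
; On success, PC_Programacion on player 0 shows the victory screen.
; Otherwise, a TextRender displays how many coins are still missing, then hides after a delay.
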(event `self.Box.OnComponentBeginOverlap`
  (params (OverlappedComponent :type "PrimitiveComponent Object Reference") (OtherActor :type "Actor Object Reference") (OtherComp :type "PrimitiveComponent Object Reference") (OtherBodyIndex :type Integer) (bFromSweep :type Boolean) (SweepResult :type "HitResult Structure (by ref)"))
  (bind _textrender (`self.TextRender`))
  (`/Game/BluePrints/Libraries/BML_Comunes.IsCharacter` OtherActor
    (:`isCharacter`
      (bind _asgm_programacion (cast `/Game/BluePrints/Core/GM_Programacion` (`GameplayStatics.GetGameMode`)))
      (bind (_gano_ _diferencia) (`/Game/BluePrints/Core/GM_Programacion.Tiene monedas para ganar?` _asgm_programacion))
      (if _gano_
        (bind _aspc_programacion (cast `/Game/BluePrints/Core/PC_Programacion` (`GameplayStatics.GetPlayerController` 0)))
        (`/Game/BluePrints/Core/PC_Programacion.Mostrar pantalla de victoria` _aspc_programacion)
        (else
          (`TextRenderComponent.K2_SetText` _textrender (`KismetSystemLibrary.MakeLiteralText` (`KismetTextLibrary.Conv_StringToText` (`KismetStringLibrary.Concat_StrStr` "Te falta recolectar " (`KismetStringLibrary.Conv_IntToString` _diferencia) " monedas para finalizar"))))
          (`SceneComponent.SetVisibility` _textrender true false)
          (`KismetSystemLibrary.Delay` 10.0)
          (`SceneComponent.SetVisibility` (`self.TextRender`) false false))))))

(fn `UserConstructionScript`)