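; BP_BaladeCañon is a cannonball actor that damages characters it touches.
; On BeginPlay it caches the damage index data from GI_Programacion, the game instance.
; When its sphere overlaps a character, it applies random damage between its minimum and maximum, scaled by that index, then spawns an explosion particle and destroys itself.
; Overlaps are filtered through IsCharacter, and the graphs contain no movement logic.
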(event `self.ReceiveBeginPlay`
  (bind _asgi_programacion (cast `/Game/BluePrints/Core/GI_Programacion` (`GameplayStatics.GetGameInstance`)))
  (set `self.Indice Daño Data` (`/Game/BluePrints/Core/GI_Programacion.Indice Daño Data` _asgi_programacion)))

(event `self.Sphere.OnComponentBeginOverlap`
  (params (OverlappedComponent :type "PrimitiveComponent Object Reference") (OtherActor :type "Actor Object Reference") (OtherComp :type "PrimitiveComponent Object Reference") (OtherBodyIndex :type Integer) (bFromSweep :type Boolean) (SweepResult :type "HitResult Structure (by ref)"))
  (bind (`_indice_daño_data_nombre` `_indice_daño_data_nombreamostrar` `_indice_daño_data_indicedaño`) (break `/Game/Data/S_IndiceDeDaño` (`self.Indice Daño Data`)))
  (`/Game/BluePrints/Libraries/BML_Comunes.IsCharacter` OtherActor
    (:`isCharacter`
      (`GameplayStatics.ApplyDamage` OtherActor (* (`KismetMathLibrary.RandomFloatInRange` (`self.Daño Minimo`) (`self.Daño Maximo`)) `_indice_daño_data_indicedaño`))
      (`GameplayStatics.SpawnEmitterAtLocation` "/Game/StarterContent/Particles/P_Explosion.P_Explosion" (`self.K2_GetActorLocation`))
      (`self.K2_DestroyActor`))))

(fn `UserConstructionScript`)