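; BP_Cañon is a cannon that fires projectiles automatically and continuously at random intervals.
; On BeginPlay it copies the IndiceDañoData settings from GI_Programacion, which supply the minimum and maximum delay between shots.
; Tick feeds a random-length Delay, acting as a repeating timer.
; After each delay it spawns a TipoDeBala actor at the PuntoDeLanzamiento transform and a P_Explosion particle effect at that location.
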(event `self.ReceiveBeginPlay`
  (bind _asgi_programacion (cast `/Game/BluePrints/Core/GI_Programacion` (`GameplayStatics.GetGameInstance`)))
  (set `self.Indice Daño Data` (`/Game/BluePrints/Core/GI_Programacion.Indice Daño Data` _asgi_programacion)))

(event `self.ReceiveTick`
  (params (DeltaSeconds :type "Float (single-precision)"))
  (bind (`_indice_daño_data_nombre` `_indice_daño_data_nombreamostrar` `_indice_daño_data_indicedaño` `_indice_daño_data_velocidadrangomin` `_indice_daño_data_velocidadrangomax`) (break `/Game/Data/S_IndiceDeDaño` (`self.Indice Daño Data`)))
  (bind _returnvalue (`SceneComponent.K2_GetComponentToWorld` (`self.Punto de Lanzamiento`)))
  (`KismetSystemLibrary.Delay` (`KismetMathLibrary.RandomFloatInRange` `_indice_daño_data_velocidadrangomin` `_indice_daño_data_velocidadrangomax`))
  (`|SpawnActorFromClass` (`self.Tipo de Bala`) _returnvalue "Undefined" "MultiplyWithRoot" null null)
  (`GameplayStatics.SpawnEmitterAtLocation` "/Game/StarterContent/Particles/P_Explosion.P_Explosion" (.location _returnvalue)))

(fn `UserConstructionScript`)