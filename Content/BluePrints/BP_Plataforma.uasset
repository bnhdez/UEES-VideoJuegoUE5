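; BP_Plataforma is a moving platform that changes color while a character stands in its trigger.
; The construction script sets InterpToMovement to travel from its origin to a configurable relative control point over a configurable duration.
; Box overlap events filter actors through an IsCharacter check, switching the Cube material to yellow on entry and back to blue on exit.
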(event `self.Box.OnComponentBeginOverlap`
  (params (OverlappedComponent :type "PrimitiveComponent Object Reference") (OtherActor :type "Actor Object Reference") (OtherComp :type "PrimitiveComponent Object Reference") (OtherBodyIndex :type Integer) (bFromSweep :type Boolean) (SweepResult :type "HitResult Structure (by ref)"))
  ; Ingresan a la colision (Estimulo)
  ; Evaluar si es jugador
  (`/Game/BluePrints/Libraries/BML_Comunes.IsCharacter` OtherActor
    (:`isCharacter`
      ; Accion
      (`PrimitiveComponent.SetMaterial` (`self.Cube`) 0 "/Game/LevelPrototyping/Materials/MI_Solid_Yellow.MI_Solid_Yellow"))))

(event `self.Box.OnComponentEndOverlap`
  (params (OverlappedComponent :type "PrimitiveComponent Object Reference") (OtherActor :type "Actor Object Reference") (OtherComp :type "PrimitiveComponent Object Reference") (OtherBodyIndex :type Integer))
  ; Salen de la colision (Estimulo)
  ; Evaluar si es jugador
  (`/Game/BluePrints/Libraries/BML_Comunes.IsCharacter` OtherActor
    (:`isCharacter`
      ; Accion
      (`PrimitiveComponent.SetMaterial` (`self.Cube`) 0 "/Game/LevelPrototyping/Materials/MI_Solid_Blue.MI_Solid_Blue"))))

(fn `UserConstructionScript`
  (bind _interptomovement (`self.InterpToMovement`))
  (set `InterpToMovementComponent.Duration` (`self.Duration`) _interptomovement)
  (set `InterpToMovementComponent.ControlPoints` (`|MakeArray` (make `InterpControlPoint` (0.0 0.0 0.0)) (make `InterpControlPoint` (`self.Position Control Point`))) _interptomovement))