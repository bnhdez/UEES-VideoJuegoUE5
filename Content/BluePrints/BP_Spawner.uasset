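; BP_Spawner is an actor that repeatedly spawns BP_Barril barrels at one of three points.
; Tick feeds a Delay with a random duration of a few seconds, which acts as a repeating timer because the node ignores calls while pending.
; After each delay, a random switch picks PuntoA, PuntoB or PuntoC and passes its world location to InstanciarBarril, which spawns the barrel unrotated at unit scale.
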(event `self.ReceiveTick`
  (params (DeltaSeconds :type "Float (single-precision)"))
  (`KismetSystemLibrary.Delay` (`KismetMathLibrary.RandomFloatInRange` 2.0 4.0))
  (switch `int` (`KismetMathLibrary.RandomIntegerInRange` 0 2)
    (:`0`
      (bind _output_get (set `self.Punto de Spawn` (`SceneComponent.K2_GetComponentLocation` (`self.Punto A`))))
      (`self.Instanciar Barril` _output_get))
    (:`1`
      (bind _output_get_2 (set `self.Punto de Spawn` (`SceneComponent.K2_GetComponentLocation` (`self.Punto B`))))
      (`self.Instanciar Barril` _output_get_2))
    (:`2`
      (bind _output_get_3 (set `self.Punto de Spawn` (`SceneComponent.K2_GetComponentLocation` (`self.Punto C`))))
      (`self.Instanciar Barril` _output_get_3))))

(fn `UserConstructionScript`)