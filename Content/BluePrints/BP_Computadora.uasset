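; BP_Computadora is a computer Blueprint that shows a text report on an array of people (Persona) through a TextRender.
; On BeginPlay, chained events loop over the array to list each person and compute headcount, total children, child and age extremes with names for ages, and counts by sex.
; Each appends to TextoAMostrar, which is displayed last.
; The sex tally reads index 0 for every increment and printed count.
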(event `self.ReceiveBeginPlay`
  (`self.Imprimir Informacion del Array`)
  (`self.Mostrar Cantidad de Personas en el Array`)
  (`self.Suma de Hijos`)
  (`self.Max y Min Cant de Hijos`)
  (`self.Max y Min de Edades`)
  (`self.Calcular Cantidades por Sexo`)
  (`self.Mostrar en Pantalla`))

(event `Imprimir Informacion del Array`
  ; Crear todo el listado
  (for _array_element (`self.Persona`)
    (`self.Imprimir Persona` _array_element)))

(event `Imprimir Persona`
  (params (Persona :type "/Game/Data/S_Persona Structure"))
  (bind (_nya `_añodenacimiento` _sexo _estado _estatura _localizacion _canthijos) (break `/Game/Data/S_Persona` Persona))
  ; Crear detalle de personas
  (set `self.Texto a Mostrar` (`KismetStringLibrary.Concat_StrStr` (`self.Texto a Mostrar`) "<br>" (`KismetStringLibrary.Concat_StrStr` "NyA: " (`KismetStringLibrary.Conv_NameToString` _nya) " | " "Año de Nacimiento: " (`KismetStringLibrary.Conv_IntToString` `_añodenacimiento`) " | " "Sexo: " (`|GetEnumeratorNameAsString` _sexo) " | " "Estatura: " (`KismetStringLibrary.Conv_DoubleToString` _estatura) " | " "Cantidad de Hijos: " (`KismetStringLibrary.Conv_ByteToString` _canthijos)))))

(event `Mostrar Cantidad de Personas en el Array`
  ; Crear cantidad de personas
  (set `self.Texto a Mostrar` (`KismetStringLibrary.Concat_StrStr` (`self.Texto a Mostrar`) "<br><br>" "Cantidad de personas: " (`KismetStringLibrary.Conv_IntToString` (`KismetArrayLibrary.Array_Length` (`self.Persona`))))))

(event `Mostrar en Pantalla`
  ; Mostrar en pantalla
  (`TextRenderComponent.K2_SetText` (`self.TextRender`) (`KismetTextLibrary.Conv_StringToText` (`self.Texto a Mostrar`))))

(event `Suma de Hijos`
  ; Suma la cantidad total de Hijos de todas las personas
  (for _array_element (`self.Persona`)
    (set `self.Suma` (+ (`self.Suma`) (`.CantHijos_20_CEE668F94A189472FE397DBCD52A9DB2` (break `/Game/Data/S_Persona` _array_element)))))
  (set `self.Texto a Mostrar` (`KismetStringLibrary.Concat_StrStr` (`self.Texto a Mostrar`) "<br><br><br>" "Suma total de Hijos: " (`KismetStringLibrary.Conv_IntToString` (`self.Suma`)))))

(event `Max y Min Cant de Hijos`
  (bind (_max_min_hijos_x _max_min_hijos_y) (break `IntPoint` (`self.Max Min HIjos`)))
  (bind (_max_min_hijos_x_2 _max_min_hijos_y_2) (break `IntPoint` (`self.Max Min HIjos`)))
  (bind (_max_min_hijos_x_3 _max_min_hijos_y_3) (break `IntPoint` (`self.Max Min HIjos`)))
  ; Maximo y Minimo total de Hijos de todas las personas
  (for _array_element (`self.Persona`)
    (`|ExecutionSequence`
      (:`then_0`
        (bind (_nya `_añodenacimiento` _sexo _estado _estatura _localizacion _canthijos) (break `/Game/Data/S_Persona` _array_element))
        (if (> _canthijos _max_min_hijos_x)
          (set `self.Max Min HIjos` (make `IntPoint` (`KismetMathLibrary.Conv_ByteToInt` _canthijos) _max_min_hijos_y))))
      (:`then_1`
        (if (< _canthijos _max_min_hijos_y_2)
          (set `self.Max Min HIjos` (make `IntPoint` _max_min_hijos_x_2 (`KismetMathLibrary.Conv_ByteToInt` _canthijos)))))))
  (set `self.Texto a Mostrar` (`KismetStringLibrary.Concat_StrStr` (`self.Texto a Mostrar`) "<br><br><br>" "La cantidad Maxima de Hijos: " (`KismetStringLibrary.Conv_IntToString` _max_min_hijos_x_3) " | " "La cantidad Minima de Hjos: " (`KismetStringLibrary.Conv_IntToString` _max_min_hijos_y_3))))

(event `Max y Min de Edades`
  (bind _returnvalue_year (`KismetMathLibrary.BreakDateTime` (`KismetMathLibrary.Now`)))
  (bind (_max_min_edad_x _max_min_edad_y) (break `IntPoint` (`self.Max Min Edad`)))
  (bind (_max_min_edad_x_2 _max_min_edad_y_2) (break `IntPoint` (`self.Max Min Edad`)))
  (bind (_max_min_edad_x_3 _max_min_edad_y_3) (break `IntPoint` (`self.Max Min Edad`)))
  ; Maximo y Minimo de edades
  (for _array_element (`self.Persona`)
    (`|ExecutionSequence`
      (:`then_0`
        (bind (_nya `_añodenacimiento`) (break `/Game/Data/S_Persona` _array_element))
        (bind _returnvalue (- _returnvalue_year `_añodenacimiento`))
        (if (> _returnvalue _max_min_edad_x)
          (set `self.Max Min Edad` (make `IntPoint` _returnvalue _max_min_edad_y))
          (set `self.Viejo` _nya)))
      (:`then_1`
        (if (< _returnvalue _max_min_edad_y_2)
          (set `self.Max Min Edad` (make `IntPoint` _max_min_edad_x_2 _returnvalue))
          (set `self.Joven` _nya)))))
  (set `self.Texto a Mostrar` (`KismetStringLibrary.Concat_StrStr` (`self.Texto a Mostrar`) "<br><br><br>" "La edad maxima es de " (`KismetStringLibrary.Conv_IntToString` _max_min_edad_x_3) " y le corresponde a " (`KismetStringLibrary.Conv_NameToString` (`self.Viejo`)) "<br>" "La edad minima es de " (`KismetStringLibrary.Conv_IntToString` _max_min_edad_y_3) " y le corresponde a " (`KismetStringLibrary.Conv_NameToString` (`self.Joven`)))))

(event `Calcular Cantidades por Sexo`
  (bind _cantidades_sexo (`self.Cantidades Sexo`))
  (bind _cantidades_sexo_2 (`self.Cantidades Sexo`))
  (bind _cantidades_sexo_3 (`self.Cantidades Sexo`))
  ; Obtener la cantidad de personas segun su sexo
  (for _array_element (`self.Persona`)
    (switch `/Game/Data/E_Sexo` (`.Sexo_21_EB3C1BE64C9503B8880B648D79523023` (break `/Game/Data/S_Persona` _array_element))
      (:`NewEnumerator0`
        (`KismetArrayLibrary.Array_Set` _cantidades_sexo_2 0 (+ (`|GetArrayItem` _cantidades_sexo_2) 1)))
      (:`NewEnumerator1`
        (`KismetArrayLibrary.Array_Set` _cantidades_sexo_3 1 (+ (`|GetArrayItem` _cantidades_sexo_3) 1)))
      (:`NewEnumerator2`
        (`KismetArrayLibrary.Array_Set` _cantidades_sexo 2 (+ (`|GetArrayItem` _cantidades_sexo) 1)))))
  (set `self.Texto a Mostrar` (`KismetStringLibrary.Concat_StrStr` (`self.Texto a Mostrar`) "<br><br><br>" "La cantidad de masculinos es de " (`KismetStringLibrary.Conv_IntToString` (`|GetArrayItem` (`self.Cantidades Sexo`))) "<br>" "La cantidad de femeninas es de " (`KismetStringLibrary.Conv_IntToString` (`|GetArrayItem` (`self.Cantidades Sexo`))) "<br>" "La cantidad de no binarios es de " (`KismetStringLibrary.Conv_IntToString` (`|GetArrayItem` (`self.Cantidades Sexo`))))))

(fn `UserConstructionScript`)