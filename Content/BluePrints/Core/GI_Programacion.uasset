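; GI_Programacion is the game instance that holds player health and difficulty-based damage data.
; On Init it reads the selected difficulty's row from DT_IndicesDeDaño and, if found, benchmarks the hardware, then applies and saves the graphics settings.
; ModificarVida adds to health, triggers PC_Programacion's death screen at zero or below, caps health at the maximum and pushes it to the UI through that controller.
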(event `self.ReceiveInit`
  (bind (_dificultad_datatable _dificultad_rowname) (break `DataTableRowHandle` (`self.Dificultad`)))
  (bind _returnvalue (`|GetDataTableRow` "/Game/Data/DT_IndicesDeDaño.DT_IndicesDeDaño" _dificultad_rowname)
    (:`then`
      (set `self.Indice Daño Data` _returnvalue)
      (bind _returnvalue_2 (`GameUserSettings.GetGameUserSettings`))
      (`GameUserSettings.LoadSettings` _returnvalue_2 false)
      (`GameUserSettings.RunHardwareBenchmark` _returnvalue_2 10 1.0 1.0)
      (`GameUserSettings.ApplyHardwareBenchmarkResults` _returnvalue_2)
      (`GameUserSettings.SaveSettings` _returnvalue_2))))

(event `Modificar Vida`
  (params (Valor :type "Float (double-precision)"))
  ; Modificar la Vida
  (bind _output_get (set `self.Vida Actual` (+ (`self.Vida Actual`) Valor)))
  (`|ExecutionSequence`
    (:`then_0`
      (if (<= _output_get 0.0)
        (bind _aspc_programacion (cast `/Game/BluePrints/Core/PC_Programacion` (`GameplayStatics.GetPlayerController` 0)))
        (`/Game/BluePrints/Core/PC_Programacion.Mostrar pantalla de muerte` _aspc_programacion)))
    (:`then_1`
      (if (> _output_get (`self.Vida Maxima`))
        (set `self.Vida Actual` (`self.Vida Maxima`)))
      (bind _aspc_programacion_2 (cast `/Game/BluePrints/Core/PC_Programacion` (`GameplayStatics.GetPlayerController` 0)))
      (`/Game/BluePrints/Core/PC_Programacion.Setear Vida en UI` _aspc_programacion_2 (`self.Vida Actual`)))))