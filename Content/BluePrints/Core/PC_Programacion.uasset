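; Player controller that owns the in-game HUD and the victory and defeat screens.
; It creates the player UI widget on BeginPlay, or lazily when an update arrives, sets game-only input, and forwards health and item count updates to it.
; Victory and defeat events share one helper that shows the given widget above the HUD, switches to UI-only input with the cursor and pauses the game.
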(event `self.ReceiveBeginPlay`
  (`self.Setup HUD`))

(event `Setear Items en la UI`
  (params (Valor :type Integer) (`Cant Ganar` :type Integer))
  ; Seteo Items
  (bind _playerui_ref (`self.PlayerUI Ref`)
    (:`then`
      _)
    (:`else`
      (`self.Setup HUD`)))
  (`/Game/UI/HUD/WBP_PlayerUI.Setear cant items` _playerui_ref Valor `Cant Ganar`))

(event `Mostrar pantalla de victoria`
  ; Pantalla de Victoria y Derrota
  (`self.Setup de pantalla de Muerte o Victoria` "/Game/UI/WBP_PatallaVictoria.WBP_PatallaVictoria_C"))

(event `Mostrar pantalla de muerte`
  ; Pantalla de Victoria y Derrota
  (`self.Setup de pantalla de Muerte o Victoria` "/Game/UI/WBP_PatallaDerrota.WBP_PatallaDerrota_C"))

(event `Setear Vida en UI`
  (params (Vida :type "Float (double-precision)"))
  ; Setear Vida en UI
  (bind _playerui_ref (`self.PlayerUI Ref`)
    (:`then`
      _)
    (:`else`
      (`self.Setup HUD`)))
  (`/Game/UI/HUD/WBP_PlayerUI.Setear Vida` _playerui_ref Vida))

(fn `Setup de pantalla de Muerte o Victoria`
  (params (Class :type "UserWidget Class Reference"))
  (bind _returnvalue (`|CreateWidget` Class))
  (`UserWidget.AddToViewport` _returnvalue 10)
  (`WidgetBlueprintLibrary.SetInputMode_UIOnlyEx` self _returnvalue)
  (set `self.bShowMouseCursor` true)
  (`GameplayStatics.SetGamePaused` true))

(fn `Setup HUD`
  (`self.PlayerUI Ref`
    (:`then`)
    (:`else`
      (bind _returnvalue (`|CreateWidget` "/Game/UI/HUD/WBP_PlayerUI.WBP_PlayerUI_C"))
      (bind _output_get (set `self.PlayerUI Ref` _returnvalue))
      (`UserWidget.AddToViewport` _output_get 0)
      (`WidgetBlueprintLibrary.SetInputMode_GameOnly` self)
      (set `self.bShowMouseCursor` false))))

(fn `UserConstructionScript`)