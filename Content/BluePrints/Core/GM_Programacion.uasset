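; GM_Programacion is a game mode that tracks collected items and decides when the player wins.
; Each pickup event increments the item count, refreshes the UI through PC_Programacion, and shows its victory screen when the count equals the target.
; It also sets the UI at BeginPlay and provides a restart event that reopens Nivel1_Level.
; A parallel coin win check is defined but not called here, and a debug win message is disconnected.
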(event `self.ReceiveBeginPlay`
  (`self.Actualizar Items en UI`))

(event `Se agarro item`
  (set `self.CantItems` (+ (`self.CantItems`) 1))
  (`self.Actualizar Items en UI`)
  (bind _gano_ (`self.Tiene items para ganar?`))
  (if _gano_
    (bind _aspc_programacion (cast `/Game/BluePrints/Core/PC_Programacion` (`GameplayStatics.GetPlayerController` 0)))
    (`/Game/BluePrints/Core/PC_Programacion.Mostrar pantalla de victoria` _aspc_programacion)))

(event `Reiniciar Nivel`
  (`GameplayStatics.OpenLevel` "Nivel1_Level"))

(fn `Tiene items para ganar?`
  (returns (`Gano?` :type Boolean) (Diferencia :type Integer))
  (bind _cantitems (`self.CantItems`))
  (bind _cantitemsganar (`self.CantItemsGanar`))
  (return (== _cantitems _cantitemsganar) (- _cantitemsganar _cantitems)))

(fn `Tiene monedas para ganar?`
  (returns (`Gano?` :type Boolean) (Diferencia :type Integer))
  (bind _cantmonedas (`self.CantMonedas`))
  (bind _cantmonedasganar (`self.CantMonedasGanar`))
  (return (== _cantmonedas _cantmonedasganar) (- _cantmonedasganar _cantmonedas)))

(fn `UserConstructionScript`)