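; BP_Item_Base is a base item actor that can be picked up when a character touches it, depending on its type.
; The construction script loads its DT_Items row by ItemID, sets the static mesh, and stops the rotation for Caja (box) items.
; On sphere overlap, Agarrable (grabbable) items notify GM_Programacion via SeAgarroItem and destroy themselves.
; Caja items only print that they cannot be grabbed.
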(event `self.Sphere.OnComponentBeginOverlap`
  (params (OverlappedComponent :type "PrimitiveComponent Object Reference") (OtherActor :type "Actor Object Reference") (OtherComp :type "PrimitiveComponent Object Reference") (OtherBodyIndex :type Integer) (bFromSweep :type Boolean) (SweepResult :type "HitResult Structure (by ref)"))
  (bind (_item_data_nombre _item_data_nombreamostrar _item_data_peso _item_data_tipo) (break `/Game/Data/S_Item` (`self.Item Data`)))
  (`/Game/BluePrints/Libraries/BML_Comunes.IsCharacter` OtherActor
    (:`isCharacter`
      (switch `/Game/Data/E_TipoDeItem` _item_data_tipo
        (:`NewEnumerator0`
          (`KismetSystemLibrary.PrintString` "No es un item agarrable"))
        (:`NewEnumerator3`
          (bind _asgm_programacion (cast `/Game/BluePrints/Core/GM_Programacion` (`GameplayStatics.GetGameMode`)))
          (`/Game/BluePrints/Core/GM_Programacion.Se agarro item` _asgm_programacion)
          (`self.K2_DestroyActor`))))))

(fn `UserConstructionScript`
  (bind _returnvalue (`|GetDataTableRow` "/Game/Data/DT_Items.DT_Items" (`self.Item ID`))
    (:`then`
      (bind _output_get (set `self.Item Data` _returnvalue))
      (`StaticMeshComponent.SetStaticMesh` (`self.StaticMesh`) (`|ConvertAsset` (`.StaticMesh_15_0F7EB51C4DC248EBEB076B9EB9216BAF` (break `/Game/Data/S_Item` _returnvalue))))
      (if (`|EnumEquality` (`.Tipo_12_5BC02D3648E7EB986DB4019630356662` (break `/Game/Data/S_Item` _output_get)) "NewEnumerator0")
        (set `RotatingMovementComponent.RotationRate` (struct) (`self.RotatingMovement`))))))