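; Player 1 dialogue trigger actor that shows a prompt and steps through an array of dialogue lines.
; When BP_player enters the Box, it reveals the TextRender and adds a Dialogo_Ui widget to the viewport; leaving reverses both.
; EventDialogo passes the Text array to the widget, shows it and advances TextRow, removing it after the last line.
; A DoOnce gate guards each advance and resets right afterwards.
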(event `self.Box.OnComponentBeginOverlap`
  (params (OverlappedComponent :type "PrimitiveComponent Object Reference") (OtherActor :type "Actor Object Reference") (OtherComp :type "PrimitiveComponent Object Reference") (OtherBodyIndex :type Integer) (bFromSweep :type Boolean) (SweepResult :type "HitResult Structure (by ref)"))
  (cast `/Game/Characters/Player/BP_player` OtherActor)
  (`SceneComponent.SetHiddenInGame` (`self.TextRender`) false false)
  (bind _returnvalue (`|CreateWidget` "/Game/Characters/Player/Dialogo/Dialogo_Ui.Dialogo_Ui_C"))
  (bind _output_get (set `self.DialogoUI` _returnvalue))
  (`UserWidget.AddToViewport` _output_get 0))

(event `self.Box.OnComponentEndOverlap`
  (params (OverlappedComponent :type "PrimitiveComponent Object Reference") (OtherActor :type "Actor Object Reference") (OtherComp :type "PrimitiveComponent Object Reference") (OtherBodyIndex :type Integer))
  (bind _dialogoui (`self.DialogoUI`))
  (cast `/Game/Characters/Player/BP_player` OtherActor)
  (`SceneComponent.SetHiddenInGame` (`self.TextRender`) true false)
  (`/Engine/EditorBlueprintResources/StandardMacros.IsValid` _dialogoui
    (:`Is Valid`
      (`Widget.RemoveFromParent` _dialogoui))))

(event `self.EventDialogo`
  (bind _dialogoui (`self.DialogoUI`))
  (bind _dialogoui_2 (`self.DialogoUI`))
  (bind _returnvalue (+ (`/Game/Characters/Player/Dialogo/Dialogo_Ui.TextRow` (`self.DialogoUI`)) 1))
  (`/Engine/EditorBlueprintResources/StandardMacros.DoOnce` false :!label _label
    (:`Completed`
      (set `/Game/Characters/Player/Dialogo/Dialogo_Ui.Text` (`self.Text`) _dialogoui_2)
      (`Widget.SetVisibility` (`/Game/Characters/Player/Dialogo/Dialogo_Ui.DialogoBorder` _dialogoui_2) "Visible")
      (`Widget.SetVisibility` (`/Game/Characters/Player/Dialogo/Dialogo_Ui.TextDialogo` _dialogoui_2) "Visible")
      (if (> _returnvalue (- (`KismetArrayLibrary.Array_Length` (`self.Text`)) 1))
        (`Widget.RemoveFromParent` _dialogoui)
        (`self.ResetDoOnce`)
        (else
          (set `/Game/Characters/Player/Dialogo/Dialogo_Ui.TextRow` _returnvalue _dialogoui)
          (`self.ResetDoOnce`))))))

(event `ResetDoOnce`
  (goto _label :!via `Reset`))

(fn `UserConstructionScript`
  (`parent.UserConstructionScript`))